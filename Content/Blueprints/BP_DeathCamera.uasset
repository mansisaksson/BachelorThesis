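; BP_DeathCamera is a camera actor, named for death views, that keeps turning to face a followed component.
; Each tick, if FollowComponent is valid, it computes the look-at rotation toward that component's world location.
; It eases the actor's rotation toward that target with a delta-time-scaled lerp, leaving its position unchanged.
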(event `self.ReceiveTick`
  (params (DeltaSeconds :type "Float (single-precision)"))
  (`/Engine/EditorBlueprintResources/StandardMacros.IsValid` (`self.FollowComponent`)
    (:`Is Valid`
      (`self.K2_SetActorRotation` (`KismetMathLibrary.RLerp` (`self.K2_GetActorRotation`) (`KismetMathLibrary.FindLookAtRotation` (`self.K2_GetActorLocation`) (`SceneComponent.K2_GetComponentLocation` (`self.FollowComponent`))) (* (`GameplayStatics.GetWorldDeltaSeconds`) 5.0))))))

(fn `UserConstructionScript`)