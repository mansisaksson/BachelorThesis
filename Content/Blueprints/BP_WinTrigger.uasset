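; Box trigger that ends the level in a win when a player character overlaps it, sized in the construction script.
; On authority it pauses the game mode timer and passes the time to EnterWinState, which shows the victory screen once, except on dedicated servers.
; EnterWinState also disables input on player 0's character, blends the view to a spawned death camera following its mesh, and turns that mesh into a physics ragdoll.
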(event `self.Box.OnComponentBeginOverlap`
  (params (OverlappedComponent :type "PrimitiveComponent Object Reference") (OtherActor :type "Actor Object Reference") (OtherComp :type "PrimitiveComponent Object Reference") (OtherBodyIndex :type Integer) (bFromSweep :type Boolean) (SweepResult :type "HitResult Structure (by ref)"))
  (cast `/Game/Blueprints/BP_PlayerCharacter` OtherActor)
  (`/Engine/EditorBlueprintResources/ActorMacros.Switch Has Authority`
    (:`Authority`
      (bind _asbp_game_mode (cast `/Game/Blueprints/BP_GameMode` (`GameplayStatics.GetGameMode`)))
      (`/Game/Blueprints/BP_GameMode.PauseTimer` _asbp_game_mode)
      (`self.Enter Win State` (`/Game/Blueprints/BP_GameMode.Timer` _asbp_game_mode)))))

(event `Enter Win State`
  (params (Time :type "Float (double-precision)"))
  (bind _explayercontroller (`/Game/Blueprints/FL_Game.GetExPlayerController`))
  (`|ExecutionSequence`
    (:`then_0`
      (`/Engine/EditorBlueprintResources/StandardMacros.DoOnce` false
        (:`Completed`
          (if (not (`KismetSystemLibrary.IsDedicatedServer`))
            (bind _returnvalue (`|CreateWidget` "/Game/Blueprints/UI/UMG_VictoryScreen.UMG_VictoryScreen_C" null Time))
            (`UserWidget.AddToViewport` _returnvalue 0)))))
    (:`then_1`
      (bind _asbp_player_character (cast `/Game/Blueprints/BP_PlayerCharacter` (`GameplayStatics.GetPlayerCharacter` 0)))
      (`self.DisableInput` _asbp_player_character null)
      (bind _returnvalue_2 (`|SpawnActorFromClass` "/Game/Blueprints/BP_DeathCamera.BP_DeathCamera_C" (`SceneComponent.K2_GetComponentToWorld` (`PlayerCharacter.FPCamera` _asbp_player_character)) "AlwaysSpawn" "OverrideRootScale" null (`Character.Mesh` _asbp_player_character)))
      (`PlayerController.SetViewTargetWithBlend` _explayercontroller _returnvalue_2 0.0 "VTBlend_Linear" 0.0 false)
      (`/Game/Blueprints/BP_ExPlayerController.SetVisiblityMode` _explayercontroller true)
      (`PrimitiveComponent.SetCollisionResponseToChannel` (`Character.CapsuleComponent` _asbp_player_character) "ECC_Destructible" "ECR_Ignore")
      (bind _mesh (`Character.Mesh` _asbp_player_character))
      (`PrimitiveComponent.SetCollisionEnabled` _mesh "PhysicsOnly")
      (`PrimitiveComponent.SetSimulatePhysics` _mesh true))))

(fn `UserConstructionScript`
  (`BoxComponent.SetBoxExtent` (`self.Box`) (`self.BoxExtent`) true))