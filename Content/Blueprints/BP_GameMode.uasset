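; Game mode Blueprint that keeps a stopwatch-style timer for the game.
; Tick adds world delta seconds to the timer whenever it is not paused.
; Start, Pause, Restart and Stop functions control the pause flag, with Restart and Stop also resetting the time to zero.
; Unconnected leftover nodes would start the timer and print it as a timespan for debugging.
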(event `self.ReceiveBeginPlay`)

(event `self.ReceiveTick`
  (params (DeltaSeconds :type "Float (single-precision)"))
  (if (not (`self.IsTimerPaused`))
    (set `self.Timer` (+ (`self.Timer`) (`GameplayStatics.GetWorldDeltaSeconds`)))))

(fn `PauseTimer`
  (set `self.IsTimerPaused` true))

(fn `RestartTimer`
  (set `self.Timer` 0.0)
  (set `self.IsTimerPaused` false))

(fn `StartTimer`
  (set `self.IsTimerPaused` false))

(fn `StopTimer`
  (set `self.Timer` 0.0)
  (set `self.IsTimerPaused` true))

(fn `UserConstructionScript`)