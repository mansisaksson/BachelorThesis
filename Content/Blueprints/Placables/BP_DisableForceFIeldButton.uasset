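; A placeable one-shot button that disables every linked forcefield when pressed.
; PressButton animates the button with a timeline, permanently hides its help text and can sink the whole panel after a delay.
; OnButtonPressed calls DisableForceField on each linked forcefield, then pans the player's view to an optional camera actor and back, skipping the pan on dedicated servers.
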(event `self.ReceiveBeginPlay`
  (bind (_returnvalue_x _returnvalue_y _returnvalue_z) (`KismetMathLibrary.BreakVector` (`self.K2_GetActorLocation`)))
  (bind (_relativelocation_x _relativelocation_y _relativelocation_z) (`KismetMathLibrary.BreakVector` (`SceneComponent.RelativeLocation` (`self.Button`))))
  (set `self.DefaultButtonZ` _relativelocation_z)
  (set `self.DefaultZLocation` _returnvalue_z))

(event `PressButton`
  (bind (_returnvalue_x _returnvalue_y) (`KismetMathLibrary.BreakVector` (`self.K2_GetActorLocation`)))
  (bind (_relativelocation_x _relativelocation_y) (`KismetMathLibrary.BreakVector` (`SceneComponent.RelativeLocation` (`self.Button`))))
  (if (not (`self.HasBeenPressed`))
    (set `self.HasBeenPressed` true)
    (`self.OnButtonPressed`)
    (`|ExecutionSequence`
      (:`then_0`
        (bind (_direction _z_offset) (`Timeline|ButtonMove` :!via `PlayFromStart`)
          (:`Update`
            (`SceneComponent.K2_SetRelativeLocation` (`self.Button`) (`KismetMathLibrary.MakeVector` _relativelocation_x _relativelocation_y (+ (`self.DefaultButtonZ`) _z_offset)) false false))))
      (:`then_1`
        (if (`self.SinkAfterPress`)
          (`KismetSystemLibrary.Delay` 2.0)
          (bind (_direction_2 _z_offset_2) (`Timeline|SinkButtonPanel_Timeline` :!via `PlayFromStart`)
            (:`Update`
              (`self.K2_SetActorRelativeLocation` (`KismetMathLibrary.MakeVector` _returnvalue_x _returnvalue_y (+ (`self.DefaultZLocation`) _z_offset_2)))))))
      (:`then_2`
        (`self.SetHelpTextHidden` true)))))

(event `OnButtonPressed`
  (if (> (`KismetArrayLibrary.Array_Length` (`self.Forcefields`)) 0)
    (for _array_element (`self.Forcefields`)
      (`/Game/Blueprints/Placables/BP_Forcefield.DisableForceField` _array_element))
    (`/Engine/EditorBlueprintResources/StandardMacros.IsValid` (`self.CameraActor`)
      (:`Is Valid`
        (if (not (`KismetSystemLibrary.IsDedicatedServer`))
          (`/Game/Blueprints/BP_ExPlayerController.PanToViewTarget` (`/Game/Blueprints/FL_Game.GetExPlayerController`) (`self.CameraActor`) 0.8 1.5 0.8))))))

(fn `SetHelpTextHidden`
  (params (newHidden :type Boolean))
  (if (`self.HasBeenPressed`)
    (`SceneComponent.SetHiddenInGame` (`self.HelpText`) true false)
    (else
      (`SceneComponent.SetHiddenInGame` (`self.HelpText`) newHidden false))))

(fn `UserConstructionScript`)