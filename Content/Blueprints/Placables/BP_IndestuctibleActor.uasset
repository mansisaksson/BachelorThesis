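; Placeable indestructible actor that shows a configurable static mesh wrapped in a force-field overlay.
; The construction script applies the chosen mesh, then adds a second mesh component using the same mesh, scaled very slightly larger to avoid z-fighting.
; That shell uses the force-field material instance and is shifted by a configurable offset.
; All event graph nodes are unused; no indestructibility logic appears here.
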(fn `UserConstructionScript`
  (`StaticMeshComponent.SetStaticMesh` (`self.StaticMesh`) (`self.Mesh`))
  (bind _returnvalue (`AddComponent|NODE_AddStaticMeshComponent-0`))
  (`SceneComponent.SetWorldScale3D` _returnvalue (+ (`SceneComponent.K2_GetComponentScale` (`self.StaticMesh`)) 0.001))
  (`StaticMeshComponent.SetStaticMesh` _returnvalue (`self.Mesh`))
  (`PrimitiveComponent.SetMaterial` _returnvalue 0 "/Game/Assets/Materials/M_ForceField_Inst.M_ForceField_Inst")
  (`SceneComponent.K2_SetRelativeLocation` _returnvalue (`self.ForceFieldOffset`) false false))