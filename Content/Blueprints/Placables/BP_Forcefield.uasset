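; BP_Forcefield is a placeable force field that can be switched off with a fade-out.
; The construction script applies the chosen mesh and pushes the color and fade toggle into its material parameters.
; DisableForceField broadcasts the faded notification immediately, then a timeline animates material opacity and, once finished, hides the mesh and disables its collision.
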(event `DisableForceField`
  ;[1 1 1] Hides force field + disables collision
  (`self.OnForcefiledFaded`)
  (bind (_direction _1_0) (`Timeline|FadeOut` :!via `PlayFromStart`)
    (:`Update`
      (`MeshComponent.SetScalarParameterValueOnMaterials` (`self.ForceFieldMesh`) "Opacity" _1_0))
    (:`Finished`
      (`SceneComponent.SetHiddenInGame` (`self.ForceFieldMesh`) true false)
      (`PrimitiveComponent.SetCollisionEnabled` (`self.ForceFieldMesh`) "NoCollision"))))

(fn `UserConstructionScript`
  (`StaticMeshComponent.SetStaticMesh` (`self.ForceFieldMesh`) (`self.Mesh`))
  (`MeshComponent.SetScalarParameterValueOnMaterials` (`self.ForceFieldMesh`) "Fade" (`KismetMathLibrary.Conv_BoolToDouble` (`self.ShouldFade`)))
  (`MeshComponent.SetVectorParameterValueOnMaterials` (`self.ForceFieldMesh`) "Color" (`KismetMathLibrary.Conv_LinearColorToVector` (`self.Color`))))