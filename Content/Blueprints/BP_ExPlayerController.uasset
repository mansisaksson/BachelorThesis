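; Player controller that runs a timed camera pan to a given actor and back to the player character.
; PanToViewTarget blocks re-entry, disables the character's input, blends the view target out, waits, then blends back and restores input.
; SetVisiblityMode toggles owner visibility between first-person arms and weapon and third-person body and gun, showing the third-person meshes during the return blend.
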(event `PanToViewTarget`
  (params (Actor :type "Actor Object Reference") (PanSpeed :type "Float (double-precision)") (WaitTime :type "Float (double-precision)") (ReturnSpeed :type "Float (double-precision)"))
  ;[1 1 1] Pan camera to view actor and then back again
  (if (not (`self.IsPanning`))
    (set `self.IsPanning` true)
    (`self.DisableInput` (`GameplayStatics.GetPlayerCharacter` 0) self)
    (`self.SetViewTargetWithBlend` Actor PanSpeed)
    (`KismetSystemLibrary.Delay` (+ PanSpeed WaitTime))
    (`self.SetVisiblityMode` false)
    (`self.SetViewTargetWithBlend` (`GameplayStatics.GetPlayerCharacter` 0) ReturnSpeed)
    (`KismetSystemLibrary.Delay` ReturnSpeed)
    (`self.EnableInput` (`GameplayStatics.GetPlayerCharacter` 0) self)
    (set `self.IsPanning` false)
    (`self.SetVisiblityMode` true)))

(fn `SetVisiblityMode`
  (params (`First/Third Person` :type Boolean))
  (locals (`First/Third Person_Local` :type Boolean))
  (set `local.First/Third Person_Local` `First/Third Person`)
  (bind _asbp_player_character (cast `/Game/Blueprints/BP_PlayerCharacter` (`GameplayStatics.GetPlayerCharacter` 0)))
  (`PrimitiveComponent.SetOwnerNoSee` (`Character.Mesh` _asbp_player_character) (`local.First/Third Person_Local`))
  (`PrimitiveComponent.SetOwnerNoSee` (`/Game/Blueprints/BP_PlayerCharacter.ThirdPersonGunMesh` _asbp_player_character) (`local.First/Third Person_Local`))
  (`PrimitiveComponent.SetOwnerNoSee` (`PlayerCharacter.ArmMesh` _asbp_player_character) (not (`local.First/Third Person_Local`)))
  (`PrimitiveComponent.SetOwnerNoSee` (`PlayerCharacter.WeaponMesh` _asbp_player_character) (not (`local.First/Third Person_Local`))))

(fn `UserConstructionScript`)