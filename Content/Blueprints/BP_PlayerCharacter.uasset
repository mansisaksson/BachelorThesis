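; First-person multiplayer player character that fires projectiles and presses force-field disable buttons.
; Input sends muzzle or camera transforms to server events, which spawn projectiles after a client-side cooldown gate or trace for buttons.
; Tick traces to toggle button help text and feeds location into a hack meant to sync server position to the client's.
; Sprint and debris-impulse logic is present but unwired.
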(event `self.ReceiveBeginPlay`
  (`|ExecutionSequence`
    (:`then_0`
      (if (not (`KismetSystemLibrary.IsDedicatedServer`))
        (bind _returnvalue (`|CreateWidget` "/Game/Blueprints/UI/UMG_Crosshair.UMG_Crosshair_C"))
        (`UserWidget.AddToViewport` _returnvalue 0)))
    (:`then_1`
      (`PrimitiveComponent.SetOwnerNoSee` (`self.Mesh`) true)
      (set `self.MaxWalkSpeed` (`CharacterMovementComponent.MaxWalkSpeed` (`self.CharacterMovement`))))))

(event `self.ReceiveTick`
  (params (DeltaSeconds :type "Float (single-precision)"))
  (`|ExecutionSequence`
    (:`then_0`
      (`self.UpdatePlayerPosition` (`self.K2_GetActorLocation`)))
    (:`then_1`
      (`self.TraceForButton`))))

(event `InputAction|Fire`
  (params (Key :type "Key Structure" :default "AnyKey"))
  ;[1 1 1] Fire weapon
  (:`Pressed`
    (if (`self.CanFire`)
      (`self.Fire_Server` (`SceneComponent.K2_GetComponentLocation` (`self.MuzzleLocation`)) (`SceneComponent.K2_GetComponentRotation` (`self.FPCamera`)))
      (set `self.CanFire` false)
      (`KismetSystemLibrary.Delay` 0.1)
      (set `self.CanFire` true))))

(event `UpdatePlayerPosition`
  (params (NewPos :type "Vector Structure"))
  ;[1 1 1] HACK: Sync client and server locations after what client says
  (if (> (`KismetMathLibrary.VSize` (- NewPos (`self.K2_GetActorLocation`))) 100.0)
    (`self.K2_SetActorLocation` NewPos false true)))

(event `Fire_Server`
  (params (Location :type "Vector Structure") (Rotation :type "Rotator Structure"))
  ;[1 1 1] Fire weapon
  (bind _returnvalue (`|SpawnActorFromClass` "/Game/Blueprints/BP_Projectile.BP_Projectile_C" (`KismetMathLibrary.MakeTransform` Location Rotation) "AlwaysSpawn" "OverrideRootScale"))
  (`PrimitiveComponent.IgnoreActorWhenMoving` (`Projectile.GetCollisionComp` _returnvalue) self true))

(event `Key|LeftShift`
  (params (Key :type "Key Structure" :default "AnyKey"))
  ;[1 1 1] Sprint
)

(event `SetWalkSpeed_Server`
  (params (NewSpeed :type "Float (double-precision)"))
  ;[1 1 1] Sprint
  (set `CharacterMovementComponent.MaxWalkSpeed` NewSpeed (`self.CharacterMovement`)))

(event `InputAction|Interact`
  (params (Key :type "Key Structure" :default "AnyKey"))
  ;[1 1 1] Interact
  (:`Pressed`
    (`self.Interact_Server` (`SceneComponent.K2_GetComponentLocation` (`self.FPCamera`)) (`SceneComponent.K2_GetComponentRotation` (`self.FPCamera`)))))

(event `Interact_Server`
  (params (Location :type "Vector Structure") (Rotation :type "Rotator Structure"))
  ;[1 1 1] Press Button
  (bind _outhit (`KismetSystemLibrary.LineTraceSingle` Location (+ Location (* (`KismetMathLibrary.GetForwardVector` Rotation) 200.0)) "TraceTypeQuery1"))
  (bind _asbp_disable_force_field_button (cast `/Game/Blueprints/Placables/BP_DisableForceFIeldButton` (`.HitActor` (`GameplayStatics.BreakHitResult` _outhit))))
  (if (== (`/Game/Blueprints/Placables/BP_DisableForceFIeldButton.PressCollider` _asbp_disable_force_field_button) (`.HitComponent` (`GameplayStatics.BreakHitResult` _outhit)))
    (`/Game/Blueprints/Placables/BP_DisableForceFIeldButton.PressButton` _asbp_disable_force_field_button)))

(event `TraceForButton`
  (bind _returnvalue (`SceneComponent.K2_GetComponentLocation` (`self.FPCamera`)))
  ;[1 1 1] Button Help Text
  (`/Engine/EditorBlueprintResources/StandardMacros.IsValid` (`self.LastHoveredButton`)
    (:`Is Valid`
      (`/Game/Blueprints/Placables/BP_DisableForceFIeldButton.SetHelpTextHidden` (`self.LastHoveredButton`) true)
      (set `self.LastHoveredButton` null))
    (:`Is Not Valid`
      _))
  (bind _outhit (`KismetSystemLibrary.LineTraceSingle` _returnvalue (+ _returnvalue (* (`KismetMathLibrary.GetForwardVector` (`SceneComponent.K2_GetComponentRotation` (`self.FPCamera`))) 200.0)) "TraceTypeQuery1"))
  (bind _asbp_disable_force_field_button (cast `/Game/Blueprints/Placables/BP_DisableForceFIeldButton` (`.HitActor` (`GameplayStatics.BreakHitResult` _outhit))))
  (if (== (`/Game/Blueprints/Placables/BP_DisableForceFIeldButton.PressCollider` _asbp_disable_force_field_button) (`.HitComponent` (`GameplayStatics.BreakHitResult` _outhit)))
    (bind _output_get (set `self.LastHoveredButton` _asbp_disable_force_field_button))
    (`/Game/Blueprints/Placables/BP_DisableForceFIeldButton.SetHelpTextHidden` _output_get false)))

(fn `UserConstructionScript`
  (`SceneComponent.K2_AttachToComponent` (`self.ThirdPersonGunMesh`) (`self.Mesh`) "hand_r" "KeepRelative" "KeepRelative" "KeepRelative" true))