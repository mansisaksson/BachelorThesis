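; BP_Projectile is a projectile actor that explodes when its collider hits something.
; On the authority it applies radial damage over the ExplosionRadius sphere, calls ApplyImpulse and Explode, then destroys itself.
; ApplyImpulse pushes overlapping components with a constant-falloff radial velocity change, tracking owners so each actor receives only one impulse.
; Explode skips dedicated servers, elsewhere spawning the explosion particles and sound before destroying the actor.
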(event `self.Collider.OnComponentHit`
  (params (HitComponent :type "PrimitiveComponent Object Reference") (OtherActor :type "Actor Object Reference") (OtherComp :type "PrimitiveComponent Object Reference") (NormalImpulse :type "Vector Structure") (Hit :type "HitResult Structure (by ref)"))
  ;[1 1 1] Explode on impact
  (`/Engine/EditorBlueprintResources/ActorMacros.Switch Has Authority`
    (:`Authority`
      (`GameplayStatics.ApplyRadialDamage` :`WorldContextObject` self :`BaseDamage` 1.0 :`Origin` (`.ImpactPoint` (`GameplayStatics.BreakHitResult` Hit)) :`DamageRadius` (`SphereComponent.SphereRadius` (`self.ExplosionRadius`)) :`DamageTypeClass` "/Game/Blueprints/BP_DamageType.BP_DamageType_C" :`DamageCauser` self :`DamagePreventionChannel` "ECC_WorldDynamic")
      (`self.ApplyImpulse`)
      (`self.Explode`)
      (`self.K2_DestroyActor`))))

(event `Explode`
  (bind _returnvalue (`self.K2_GetActorLocation`))
  ;[1 1 1] Explode on impact
  (if (not (`KismetSystemLibrary.IsDedicatedServer`))
    (`GameplayStatics.SpawnEmitterAtLocation` "/Game/Assets/Particles/P_Explosion.P_Explosion" _returnvalue)
    (`GameplayStatics.PlaySoundAtLocation` "/Game/Assets/Audio/Explosion_Cue.Explosion_Cue" _returnvalue)
    (`self.K2_DestroyActor`)))

(fn `ApplyImpulse`
  (locals (Actors :type "Array of Actor Object Reference"))
  (for _array_element (`PrimitiveComponent.GetOverlappingComponents` (`self.ExplosionRadius`))
    (bind _returnvalue (`ActorComponent.GetOwner` _array_element))
    (if (not (`KismetArrayLibrary.Array_Contains` (`local.Actors`) _returnvalue))
      (`PrimitiveComponent.AddRadialImpulse` _array_element (`self.K2_GetActorLocation`) (`SphereComponent.SphereRadius` (`self.ExplosionRadius`)) (`self.ExplosionStrength`) "RIF_Constant" true)
      (`KismetArrayLibrary.Array_Add` (`local.Actors`) _returnvalue))))

(fn `UserConstructionScript`)